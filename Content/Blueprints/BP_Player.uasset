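; Player pawn for a shooter that moves on the X-Z plane, fires projectile weapons and ends the game on death.
; A timeline spawn animation unlocks firing, while interpolated axis input drives swept movement, yaw tilt and bounces off hit normals.
; Looping timers repeat primary and twin secondary fire using classes from SetWeapons, though beam and charge inputs are stubs.
; Damage triggers camera shake through BP_GameMode, and zero health adds an explosion before GameOver.
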(event OnComponentHit(Box)
  (params (HitComponent :type Primitive%20Component%20Object%20Reference) (OtherActor :type Actor%20Object%20Reference) (OtherComp :type Primitive%20Component%20Object%20Reference) (NormalImpulse :type Vector :default "0, 0, 0") (Hit :type Hit%20Result%20Structure%20%28by%20ref%29))
  (bind (_x _y _z) (Math|Vector|BreakVector (.normal Hit)))
  ;[1 1 1] On Hit Bounce
  (Variables|Default|SetHozSpeed (* (* (Math|Float|Absolute(Float) (Variables|Default|GetHozSpeed)) 0.75) _x))
  (Variables|Default|SetVertSpeed (* (* (Math|Float|Absolute(Float) (Variables|Default|GetVertSpeed)) 0.75) _z)))

(event Custom|PrimeFire
  ;[1 1 1] Primary Fire
  (CallFunction|PrimaryFire (Transformation|GetWorldTransform (Variables|Default|GetProjectileSpawn))))

(event Custom|SecFire
  ;[1 1 1] Secondary Fire
  (CallFunction|SecondaryFire (Transformation|GetWorldTransform (Variables|Default|GetProjectileSpawnL)))
  (CallFunction|SecondaryFire (Transformation|GetWorldTransform (Variables|Default|GetProjectileSpawnR))))

(event EventBeginPlay
  ;[1 1 1] Player Spawn Animation
  (CallFunction|SetWeapons "NewEnumerator0")
  (bind _asbp_game_mode (Utilities|Casting|CastToBP_GameMode (Game|GetGameMode)))
  (Variables|Default|SetBP_GameMode _asbp_game_mode)
  (Variables|Default|SetYaw (.Yaw (Math|Rotator|BreakRotator (Transformation|GetActorRotation))))
  (Variables|Default|SetSpawnLocation (Transformation|GetActorLocation))
  (bind _speed (Timeline|SpawnAnimation Play)
    (:Update
      (Transformation|SetActorLocation (Math|Vector|Lerp(Vector) (Variables|Default|GetSpawnLocation) (+ (Variables|Default|GetSpawnLocation) "0,0.000000,60.000000") _speed) false false)
      (Transformation|SetRelativeRotation (Variables|Default|GetPlayerMesh) (Math|Rotator|Lerp(Rotator) "0, 0, 0" (Math|Rotator|MakeRotator 0.0 0.0 (+ (Variables|Default|GetYaw) (Variables|Default|GetSpawnSpinCount))) _speed) false false))
    (:Finished
      (Variables|Default|SetMoveEnabled true))))

(event EventTick
  (params (DeltaSeconds :type Float%20%28single-precision%29))
  (bind _playermesh (Variables|Default|GetPlayerMesh))
  ;[1 1 1] Movement and Player Input
  (Variables|Default|SetDeltaSeconds DeltaSeconds)
  (Transformation|SetActorLocation (+ (Transformation|GetActorLocation) (Math|Vector|MakeVector (Variables|Default|GetHozSpeed) 0.0 0.0)) true false)
  (Transformation|SetActorLocation (+ (Transformation|GetActorLocation) (Math|Vector|MakeVector 0.0 0.0 (Variables|Default|GetVertSpeed))) true false)
  (Utilities|IsValid self
    (:Is%20Valid
      (Transformation|SetRelativeRotation _playermesh (Class|KismetMathLibrary|RInterptoConstant (Variables|/Script/Engine.SceneComponent|GetRelativeRotation _playermesh) (Math|Rotator|MakeRotator 0.0 0.0 (+ (* (Variables|Default|GetHozSpeed) -7.0) (Variables|Default|GetYaw))) (Variables|Default|GetDeltaSeconds) 8e+01) false false))))

(event Game|Damage|EventAnyDamage
  (params (Damage :type Float%20%28single-precision%29) (DamageType :type Damage%20Type%20Object%20Reference) (InstigatedBy :type Controller%20Object%20Reference) (DamageCauser :type Actor%20Object%20Reference))
  (bind _returnvalue (Transformation|GetActorLocation))
  ;[1 1 1] Damage
  (Variables|Default|SetHealth (Math|Float|Clamp(Float) (- (Variables|Default|GetHealth) Damage) 0.0 (Variables|Default|GetMaxHealth)))
  (Default|PlayCamShake (Variables|Default|GetBP_GameMode) "/Game/Blueprints/CamShakes/BP_CamShakeSmall.BP_CamShakeSmall_C" (Transformation|GetActorLocation))
  (if (<= (Variables|Default|GetHealth) 0.0)
    (Effects|SpawnEmitteratLocation "/Game/Assets/Particles/P_Pixel_Explosion_Player.P_Pixel_Explosion_Player" _returnvalue)
    (Audio|PlaySoundatLocation 0 _returnvalue "0, 0, 0" 1.0 1.0 0.0 0 0 0)
    (Default|PlayCamShake (Variables|Default|GetBP_GameMode) "/Game/Blueprints/CamShakes/BP_CamShake.BP_CamShake_C" (Transformation|GetActorLocation))
    (Default|GameOver (Variables|Default|GetBP_GameMode))
    (Actor|DestroyActor)))

(event Input|ActionEvents|InputActionPrimaryFire
  (params (Key :type Key%20Structure))
  ;[1 1 1] Primary Fire
  (:Pressed
    (if (Variables|Default|GetMoveEnabled)
      (Utilities|Time|SetTimerbyFunctionName 0 "PrimeFire" 0.2 true)
      (CallFunction|PrimaryFire (Transformation|GetWorldTransform (Variables|Default|GetProjectileSpawn)))))
  (:Released
    (Utilities|Time|ClearTimerbyFunctionName 0 "PrimeFire")))

(event Input|ActionEvents|InputActionSecondaryFire
  (params (Key :type Key%20Structure))
  (bind _currentsecondaryweapon (Variables|Default|GetCurrentSecondaryWeapon))
  ;[1 1 1] Secondary Fire
  (:Pressed
    (switch Utilities|FlowControl|Switch|SwitchonPlayerWeapons _currentsecondaryweapon
      (:NewEnumerator1
        (if (Variables|Default|GetMoveEnabled)
          (Utilities|Time|SetTimerbyFunctionName 0 "SecFire" 0.6 true)
          (CallFunction|SecondaryFire (Transformation|GetWorldTransform (Variables|Default|GetProjectileSpawnL)))
          (CallFunction|SecondaryFire (Transformation|GetWorldTransform (Variables|Default|GetProjectileSpawnR)))))
      (:NewEnumerator2
        (if true
          _))
      (:NewEnumerator3
        (if (Variables|Default|GetMoveEnabled)
          _))))
  (:Released
    (switch Utilities|FlowControl|Switch|SwitchonPlayerWeapons _currentsecondaryweapon
      (:NewEnumerator1
        (Utilities|Time|ClearTimerbyFunctionName 0 "SecFire")))))

(event Input|AxisEvents|InputAxisMoveUpDown
  (params (AxisValue :type Float%20%28single-precision%29))
  ;[1 1 1] Movement and Player Input
  (bind _returndirectionspeed (CallFunction|Movement AxisValue (Variables|Default|GetVertSpeed)))
  (Variables|Default|SetVertSpeed _returndirectionspeed))

(event Input|AxisEvents|InputAxisMoveRightLeft
  (params (AxisValue :type Float%20%28single-precision%29))
  ;[1 1 1] Movement and Player Input
  (bind _returndirectionspeed (CallFunction|Movement AxisValue (Variables|Default|GetHozSpeed)))
  (Variables|Default|SetHozSpeed _returndirectionspeed))

(fn ConstructionScript
  (Variables|Default|SetHealth (Variables|Default|GetMaxHealth)))

(fn Movement
  (params (Direction :type Float%20%28single-precision%29) (Speed :type Float%20%28single-precision%29))
  (bind _deltaseconds (Variables|Default|GetDeltaSeconds))
  (return (Math|Interpolation|FInterpTo Speed (* (* (Variables|Default|GetMovementSpeed) Direction) _deltaseconds) _deltaseconds 5.0)))

(fn PrimaryFire
  (params (SpawnTransform :type Transform))
  (Game|SpawnActorfromClass (Variables|Default|GetPrimaryWeapon) SpawnTransform "AlwaysSpawn" 0 (LocalVariables|GetProjectileColour) self)
  (Audio|PlaySoundatLocation 0 (Transformation|GetActorLocation) "0, 0, 0" 1.0 1.0 0.0 0 0 0))

(fn SecondaryFire
  (params (Spawn :type Transform))
  (Game|SpawnActorfromClass (Variables|Default|GetSecondaryWeapon) Spawn "AlwaysSpawn" 0 (LocalVariables|GetColour) 0)
  (Audio|PlaySoundatLocation 0 (Transformation|GetActorLocation) "0, 0, 0" 1.0 1.0 0.0 0 0 0))

(fn SetWeapons
  (params (WeaponType :type PlayerWeapons%20Enum :default "NewEnumerator0"))
  (switch Utilities|FlowControl|Switch|SwitchonPlayerWeapons WeaponType
    (:NewEnumerator0
      (Variables|Default|SetPrimaryWeapon "/Game/Blueprints/Projectiles/PlayerProjectile/BP_ProjectilePlayerPrimary.BP_ProjectilePlayerPrimary_C"))
    (:NewEnumerator1
      (Variables|Default|SetSecondaryWeapon "/Game/Blueprints/Projectiles/PlayerProjectile/BP_ProjectilePlayerSecondary.BP_ProjectilePlayerSecondary_C")
      (Variables|Default|SetCurrentSecondaryWeapon WeaponType :!label _label))
    (:NewEnumerator2
      (Variables|Default|SetSecondaryWeapon "/Game/Blueprints/Projectiles/PlayerProjectile/BP_BeamProjectile.BP_BeamProjectile_C")
      (goto _label))
    (:NewEnumerator3
      (Variables|Default|SetSecondaryWeapon "/Game/Blueprints/Projectiles/PlayerProjectile/BP_ChargeProjectile.BP_ChargeProjectile_C")
      (goto _label))))