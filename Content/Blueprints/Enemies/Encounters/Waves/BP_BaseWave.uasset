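; Base enemy wave for encounters that spawns a list of enemy classes and tracks when all are killed.
; SpawnWave's Circle rule spaces enemies by pitch angle on a vertical ring around a fixed world-space point, not the wave's location, and gives each a reference back to the wave.
; RemoveEnemy counts kills and calls RemoveWave on the owning encounter once the count matches the list length.
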(event EventBeginPlay)

(event Collision|EventActorBeginOverlap
  (params (OtherActor :type Actor%20Object%20Reference)))

(event EventTick
  (params (DeltaSeconds :type Float%20%28single-precision%29)))

(fn ConstructionScript)

(fn SpawnWave
  (bind _enemies (Variables|Default|GetEnemies))
  (switch Utilities|FlowControl|Switch|SwitchonSpawnRules (Variables|Default|GetSpawnRule)
    (:NewEnumerator1
      (for (_array_element _array_index) _enemies
        (bind _returnvalue (Game|SpawnActorfromClass _array_element (Math|Transform|MakeTransform (+ (* (Math|Vector|GetForwardVector (Math|Rotator|MakeRotator 0.0 (Math|Conversions|ToFloat(Integer) (* _array_index (/ 360 (Utilities|Array|Length _enemies)))) 0.0)) 1e+02) "0,100.000000,200.000000") "0, 0, 0" "1,1,1") "Undefined" 0 0))
        (Variables|/Game/Blueprints/Enemies/BP_EnemyBase.BP_EnemyBase_C|SetWave _returnvalue self)))))

(fn RemoveEnemy
  (bind _result (Math|Integer|IncrementInt (Variables|Default|GetEnemiesKilled))
    (:%20%20
      (if (== (Utilities|Array|Length (Variables|Default|GetEnemies)) _result)
        (Default|RemoveWave (Variables|Default|GetEncounterRef))))))