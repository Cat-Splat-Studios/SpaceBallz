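; BP_BaseEncouter is a base enemy encounter that runs a list of wave actor classes in sequence.
; SpawnEncounter spawns the indexed wave at the encounter's transform, calls its SpawnWave and then hands it a reference back to the encounter.
; RemoveWave advances the finished count and spawns the next wave, or, after the last, increments the spawner's EncountersFinished and calls its Spawn.
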(event EventBeginPlay)

(event Collision|EventActorBeginOverlap
  (params (OtherActor :type Actor%20Object%20Reference)))

(event EventTick
  (params (DeltaSeconds :type Float%20%28single-precision%29)))

(fn ConstructionScript)

(fn SpawnEncounter
  (params (Index :type Integer))
  (bind _returnvalue (Game|SpawnActorfromClass (Utilities|Array|Get(acopy) (Variables|Default|GetWaves) Index) (Transformation|GetActorTransform) "Undefined" 0 0))
  (Default|SpawnWave _returnvalue)
  (Variables|/Game/Blueprints/Enemies/Encounters/Waves/BP_BaseWave.BP_BaseWave_C|SetEncounterRef _returnvalue self))

(fn RemoveWave
  (bind _wavesfinished (Variables|Default|GetWavesFinished))
  (bind _spawnerref (Variables|Default|GetSpawnerRef))
  (bind _result (Math|Integer|IncrementInt _wavesfinished)
    (:%20%20
      (if (== (Utilities|Array|Length (Variables|Default|GetWaves)) _result)
        (Math|Integer|IncrementInt (Variables|/Game/Blueprints/Enemies/BP_EnemySpawner.BP_EnemySpawner_C|GetEncountersFinished _spawnerref)
          (:%20%20
            (Default|Spawn _spawnerref)))
        (else
          (CallFunction|SpawnEncounter _wavesfinished))))))