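; Game mode that tracks score, top score, currency, enemy counts and level progression, and shows the HUD and Game Over screen.
; BeginPlay restores state from a save slot; EndPlay resets score and level progress before saving, so top score and currency carry over.
; LoadLevel opens Level_1 first, picks randomly among uncompleted middle levels, then opens Level_5 once four are completed.
; Helper functions open the shop and play world camera shakes.
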(event EventBeginPlay
  (Input|SetInputModeGameOnly (Game|GetPlayerController 0))
  (CallFunction|LoadState)
  (bind _returnvalue (UserInterface|CreateWidget "/Game/Blueprints/Hud_UI/BPW_HUD.BPW_HUD_C"))
  (bind _output_get (Variables|Default|SetBPW_HUD _returnvalue))
  (UserInterface|Viewport|AddtoViewport _output_get 0))

(event EventEndPlay
  (params (EndPlayReason :type EEndPlayReason%20Enum :default "Destroyed"))
  (CallFunction|ResetLevels)
  (CallFunction|SaveState))

(fn ConstructionScript)

(fn LoadState
  (SaveGame|DoesSaveGameExist "Slot 1")
  (if true
    (bind _returnvalue (SaveGame|LoadGamefromSlot "Slot 1"))
    (bind _asbp_save_state (Utilities|Casting|CastToBP_SaveState _returnvalue))
    (Variables|Default|SetTopScore (Variables|/Game/Blueprints/BP_SaveState.BP_SaveState_C|GetSaved_TopScore _asbp_save_state))
    (Variables|Default|SetCurrency (Variables|/Game/Blueprints/BP_SaveState.BP_SaveState_C|GetSaved_Currency _asbp_save_state))
    (Variables|Default|SetLevelsCompleted (Variables|/Game/Blueprints/BP_SaveState.BP_SaveState_C|GetSaved_LevelsCompleted _asbp_save_state))
    (Variables|Default|SetScore (Variables|/Game/Blueprints/BP_SaveState.BP_SaveState_C|GetSaved_CurrentScore _asbp_save_state))
    (Variables|Default|SetLevel_1_Complete (Variables|/Game/Blueprints/BP_SaveState.BP_SaveState_C|GetSaved_Level_1 _asbp_save_state))
    (Variables|Default|SetLevel_2_Complete (Variables|/Game/Blueprints/BP_SaveState.BP_SaveState_C|GetSaved_Level_2 _asbp_save_state))
    (Variables|Default|SetLevel_3_Complete (Variables|/Game/Blueprints/BP_SaveState.BP_SaveState_C|GetSaved_Level_3 _asbp_save_state))
    (Variables|Default|SetLevel_4_Complete (Variables|/Game/Blueprints/BP_SaveState.BP_SaveState_C|GetSaved_Level_4 _asbp_save_state))
    (else
      (Development|PrintString "No Data Dummy"))))

(fn SaveState
  (bind _returnvalue (SaveGame|CreateSaveGameObject "/Game/Blueprints/BP_SaveState.BP_SaveState_C"))
  (bind _output_get (Variables|Default|SetSave_Ref _returnvalue))
  ;[1 1 1] Top Score
  (bind _output_get_2 (Variables|Default|SetTopScore (Variables|Default|GetTopScore)))
  (Variables|/Game/Blueprints/BP_SaveState.BP_SaveState_C|SetSaved_TopScore _output_get _output_get_2)
  ;[1 1 1] Currency
  (bind _output_get_3 (Variables|Default|SetCurrency (Variables|Default|GetCurrency)))
  (Variables|/Game/Blueprints/BP_SaveState.BP_SaveState_C|SetSaved_Currency _output_get _output_get_3)
  ;[1 1 1] Levels Completed
  (bind _output_get_4 (Variables|Default|SetLevelsCompleted (Variables|Default|GetLevelsCompleted)))
  (Variables|/Game/Blueprints/BP_SaveState.BP_SaveState_C|SetSaved_LevelsCompleted _output_get _output_get_4)
  ;[1 1 1] Current Score
  (bind _output_get_5 (Variables|Default|SetScore (Variables|Default|GetScore)))
  (bind _output_get_6 (Variables|/Game/Blueprints/BP_SaveState.BP_SaveState_C|SetSaved_CurrentScore _output_get _output_get_5))
  (bind _output_get_7 (Variables|Default|SetLevel_1_Complete (Variables|Default|GetLevel_1_Complete)))
  (Variables|/Game/Blueprints/BP_SaveState.BP_SaveState_C|SetSaved_Level_1 _output_get _output_get_7)
  (bind _output_get_8 (Variables|Default|SetLevel_2_Complete (Variables|Default|GetLevel_2_Complete)))
  (Variables|/Game/Blueprints/BP_SaveState.BP_SaveState_C|SetSaved_Level_2 _output_get _output_get_8)
  (bind _output_get_9 (Variables|Default|SetLevel_3_Complete (Variables|Default|GetLevel_3_Complete)))
  (Variables|/Game/Blueprints/BP_SaveState.BP_SaveState_C|SetSaved_Level_3 _output_get _output_get_9)
  (bind _output_get_10 (Variables|Default|SetLevel_4_Complete (Variables|Default|GetLevel_4_Complete)))
  (Variables|/Game/Blueprints/BP_SaveState.BP_SaveState_C|SetSaved_Level_4 _output_get _output_get_10)
  (SaveGame|SaveGametoSlot _returnvalue "Slot 1" _output_get_6))

(fn SetScore
  (params (A :type Integer))
  (bind _output_get (Variables|Default|SetScore (+ A (Variables|Default|GetScore))))
  (if (>= _output_get (Variables|Default|GetTopScore))
    (Variables|Default|SetTopScore (Variables|Default|GetScore))
    (else
      (Variables|Default|SetTopScore (Variables|Default|GetTopScore)))))

(fn UpdateEnemyCount
  (params (Val :type Integer))
  (Variables|Default|SetEnemyCount (+ Val (Variables|Default|GetEnemyCount))))

(fn PlayCamShake
  (params (Shake :type Camera%20Shake%20Class%20Reference) (Epicenter :type Vector))
  (Camera|PlayWorldCameraShake Shake Epicenter 0.0 1e+03))

(fn GameOver
  (bind _returnvalue (Game|GetPlayerController 0))
  (bind _returnvalue_2 (UserInterface|CreateWidget "/Game/Blueprints/Hud_UI/BPW_GameOver.BPW_GameOver_C"))
  (UserInterface|Viewport|AddtoViewport _returnvalue_2 0)
  (Variables|/Script/Engine.PlayerController|SetbShowMouseCursor _returnvalue true)
  (Input|SetInputModeUIOnly _returnvalue _returnvalue_2 "DoNotLock")
  (CallFunction|ResetLevels))

(fn EnemyKilled
  (Math|Integer|IncrementInt (Variables|Default|GetEnemiesKilled)
    (:%20%20
      (CallFunction|UpdateEnemyCount -1))))

(fn GetCurrency
  (params (A :type Integer))
  (Variables|Default|SetCurrency (+ A (Variables|Default|GetCurrency))))

(fn LoadShop
  (Game|OpenLevel(byName) "Shop"))

(fn LoadLevel
  (bind _randomlevels (Variables|Default|GetRandomLevels))
  (if (Variables|Default|GetLevel_1_Complete)
    (if (== (Variables|Default|GetLevelsCompleted) 4)
      (Game|OpenLevel(byName) "Level_5")
      (else
        (if (Variables|Default|GetLevel_2_Complete)
          (Utilities|Array|RemoveItem _randomlevels "Level_2"))
        (if (Variables|Default|GetLevel_3_Complete)
          (Utilities|Array|RemoveItem _randomlevels "Level_3"))
        (if (Variables|Default|GetLevel_4_Complete)
          (Utilities|Array|RemoveItem _randomlevels "Level_4"))
        (Game|OpenLevel(byName) (Utilities|String|StringToName (Utilities|Array|Get(acopy) _randomlevels (Math|Random|RandomInteger (Utilities|Array|Length _randomlevels)))))))
    (else
      (Game|OpenLevel(byName) "Level_1"))))

(fn ResetLevels
  (Variables|Default|SetLevelsCompleted 0)
  (Variables|Default|SetScore 0)
  (Variables|Default|SetLevel_1_Complete false)
  (Variables|Default|SetLevel_2_Complete false)
  (Variables|Default|SetLevel_3_Complete false)
  (Variables|Default|SetLevel_4_Complete false)
  (Variables|Default|SetLevel_5_Complete false))